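; AI controller that steers its pawn through a labyrinth with constant movement input until IsLabyrinthCompleted is true.
; Each Tick traces ahead on Visibility; on a hit, a second, shorter trace picks which way to yaw the movement Direction.
; The trace helper ignores its angle input, so the intended right-side probe also points along the pawn's forward vector.
; The left probe is never run.
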(event `self.ReceiveTick`
  (params (DeltaSeconds :type "Float (single-precision)"))
  (if (not (`self.IsLabyrinthCompleted`))
    (bind _returnvalue (`self.CustomLineTraceByChannel` 100 (`self.LineTraceDegForward`)))
    (if _returnvalue
      (bind _returnvalue_2 (`self.CustomLineTraceByChannel` 75 (`self.LineTraceDegRight`)))
      (bind _output_get (set `self.Direction` (`KismetMathLibrary.GreaterGreater_VectorRotator` (`self.Direction`) (`KismetMathLibrary.MakeRotator` 0.0 0.0 (select `bool` _returnvalue_2 :`false` 20.0 :`true` -20.0 :!type "Float (single-precision)"))))))
    (`Pawn.AddMovementInput` (`self.K2_GetPawn`) _output_get 1.0 false)))

(fn `CustomLineTraceByChannel`
  (params (`Line Trace Length` :type Integer) (`Line Trace Angle (Deg)` :type "Float (double-precision)"))
  (returns (ReturnValue :type Boolean) (`Out Hit Distance` :type "Float (double-precision)"))
  (locals (NewLocalVar_0 :type "HitResult Structure"))
  (bind _returnvalue (`self.K2_GetPawn`))
  (bind _returnvalue_2 (`self.K2_GetActorLocation` _returnvalue))
  (bind (_outhit _returnvalue_3) (`KismetSystemLibrary.LineTraceSingle` :`Start` _returnvalue_2 :`End` (+ _returnvalue_2 (* (`self.GetActorForwardVector` _returnvalue) `Line Trace Length`)) :`TraceChannel` "TraceTypeQuery1" :`DrawDebugType` "ForOneFrame"))
  (return _returnvalue_3 (`.Distance` (`GameplayStatics.BreakHitResult` _outhit))))

(fn `UserConstructionScript`)